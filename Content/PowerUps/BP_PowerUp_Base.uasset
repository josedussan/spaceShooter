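; Base power-up pickup actor that spins, travels forward and is collected by the player on overlap.
; BeginPlay applies a configurable rate to one axis of its RotatingMovement component, and Tick moves it along its forward vector at Speed without sweeping.
; Overlap with an actor tagged "Player" spawns an emitter, plays a collect sound and destroys the pickup after a short delay.
; No gameplay effect is granted here.
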(event `self.ReceiveBeginPlay`
  (set `RotatingMovementComponent.RotationRate` (`KismetMathLibrary.MakeRotator` (`self.RotationRate`)) (`self.RotatingMovement`)))

(event `self.ReceiveActorBeginOverlap`
  (params (OtherActor :type "Actor Object Reference"))
  (if (`KismetArrayLibrary.Array_Contains` (`Actor.Tags` OtherActor) "Player")
    (`GameplayStatics.SpawnEmitterAtLocation` null)
    (`GameplayStatics.PlaySound2D` "/Game/Fab/Free_Sounds_Pack/cue/Special_Collectible_26-1_Cue.Special_Collectible_26-1_Cue" 1.0 1.0 0.0 null null)
    (`KismetSystemLibrary.Delay` 0.2)
    (`self.K2_DestroyActor`)))

(event `self.ReceiveTick`
  (params (DeltaSeconds :type "Float (single-precision)"))
  (`self.K2_SetActorLocation` (+ (`self.K2_GetActorLocation`) (* (`self.GetActorForwardVector`) (* DeltaSeconds (`self.Speed`))))))

(fn `UserConstructionScript`)