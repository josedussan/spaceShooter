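; BP_EnemeyG is a child enemy Blueprint that spins through a RotatingMovement component and customizes behavior inherited from its parent.
; On BeginPlay it runs the parent logic, sets the rotation rate from RotacionZ, overrides DelayShoot and plays a sci-fi shot sound in 2D.
; It contains no firing logic of its own, and its construction script only calls the parent.
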(event `self.ReceiveBeginPlay`
  (`parent.ReceiveBeginPlay`)
  (set `RotatingMovementComponent.RotationRate` (`KismetMathLibrary.MakeRotator` (`self.rotacionZ`)) (`self.RotatingMovement`))
  (set `self.DelayShoot` 1.0)
  (`GameplayStatics.PlaySound2D` "/Game/Fab/Sci-Fi_Shots_Pack2_Game_Of_Weapons/Cue/SciFi_Shot_P2__70__Cue.SciFi_Shot_P2__70__Cue" 1.0 1.0 0.0 null null))

(fn `UserConstructionScript`
  (`parent.UserConstructionScript`))