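; BP_EnemyH is an enemy variant that sets a horizontal movement direction along its right vector, starting rightward.
; Overlapping any actor without the "Enemy" tag flips MovementVector between right and left, tracked by IsRight.
; Each flip from right to left also shortens DelayShoot slightly.
; Tick only calls the parent, so this graph sets the direction but does not apply movement or shooting itself.
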(event `self.ReceiveBeginPlay`
  (`parent.ReceiveBeginPlay`)
  (set `self.MovementVector` (`self.GetActorRightVector`))
  (set `self.IsRight` true))

(event `self.ReceiveActorBeginOverlap`
  (params (OtherActor :type "Actor Object Reference"))
  (bind _returnvalue (`self.GetActorRightVector`))
  (`parent.ReceiveActorBeginOverlap` OtherActor)
  (`KismetSystemLibrary.PrintString` "colisiona")
  (if (`KismetArrayLibrary.Array_Contains` (`Actor.Tags` OtherActor) "Enemy")
    _
    (elif (`self.IsRight`)
      (set `self.IsRight` false)
      (set `self.MovementVector` (* _returnvalue (-1.0 -1.0 -1.0)))
      (set `self.DelayShoot` (- (`self.DelayShoot`) 0.1))
      (else
        (set `self.IsRight` true)
        (set `self.MovementVector` _returnvalue)))))

(event `self.ReceiveTick`
  (params (DeltaSeconds :type "Float (single-precision)"))
  (`parent.ReceiveTick` DeltaSeconds))

(fn `UserConstructionScript`
  (`parent.UserConstructionScript`))