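; BP_EnemyAmmo is an enemy projectile that flies straight and explodes when it overlaps an actor tagged Player.
; Tick moves it along its forward vector by Speed scaled by delta time, without sweeping.
; On a Player overlap it spawns a half-scale explosion emitter and destroys itself after a brief delay, applying no damage in this graph.
; An alternative Pawn-cast check is left disconnected and never runs.
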(event `self.ReceiveBeginPlay`)

(event `self.ReceiveActorBeginOverlap`
  (params (OtherActor :type "Actor Object Reference"))
  (if (`KismetArrayLibrary.Array_Contains` (`Actor.Tags` OtherActor) "Player")
    (`GameplayStatics.SpawnEmitterAtLocation` "/Game/StarterContent/Particles/P_Explosion.P_Explosion" (`self.K2_GetActorLocation`) (struct) (0.5 0.5 0.5))
    (`KismetSystemLibrary.Delay` 0.1)
    (`self.K2_DestroyActor`)))

(event `self.ReceiveTick`
  (params (DeltaSeconds :type "Float (single-precision)"))
  (`self.K2_SetActorLocation` (+ (`self.K2_GetActorLocation`) (* (`self.GetActorForwardVector`) (* DeltaSeconds (`self.speed`))))))

(fn `UserConstructionScript`)